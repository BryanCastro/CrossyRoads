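; Logs_BP is an actor that moves a randomly chosen log mesh along a spline in an endless loop.
; BeginPlay picks the mesh, caches the start position and an otherwise unused Vehicle_BP reference, then calls MoveObject.
; A timeline scaled by TimeToCompleteS drives the actor along the spline.
; Each pass randomly favors a 180-degree flipped placement over a Y-offset one, then resets after a short delay.
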(event Custom|MoveObject
  (bind _spline (Variables|Default|Getspline))
  (bind _start_position (Variables|Default|GetStart_position))
  (Components|Timeline|SetPlayRate (Variables|Default|GetMove%20Object%20T) (/ 1.0 (Variables|Default|GetTime%20To%20Complete%28s%29)))
  (if (> (Math|Random|RandomInteger 3) 0) :!label _label
    (Variables|Default|SetRotation "0,180.000000, 0")
    (Transformation|SetActorTransform (Math|Transform|MakeTransform (+ _start_position "0,0.000000, 0") "0,180.000000, 0" "1,1,1"))
    (bind _move_track (Timeline|Move%20Object%20T PlayFromStart)
      (:Update
        (Transformation|SetActorLocation (Spline|GetLocationatDistanceAlongSpline _spline (Math|Float|Lerp 0.0 (Spline|GetSplineLength _spline) _move_track) "World") false false))
      (:Finished
        (Transformation|SetWorldLocation (Variables|Default|GetDefaultSceneRoot) _start_position false false)
        (Utilities|FlowControl|Delay 0.2)
        (goto _label)))
    (else
      (Variables|Default|SetRotation "0, 0, 0")
      (Transformation|SetActorTransform (Math|Transform|MakeTransform (+ _start_position "0,1900.000000, 0") "0, 0, 0" "1,1,1"))
      (Timeline|Move%20Object%20T PlayFromStart))))

(event EventBeginPlay
  (bind _returnvalue (Actor|GetActorOfClass "/Game/blueprints/Vehicle_BP.Vehicle_BP_C"))
  (Variables|Default|SetNewVar_0 _returnvalue)
  (Variables|Default|SetStart_position (Transformation|GetWorldLocation (Variables|Default|GetDefaultSceneRoot)))
  (bind _output_get (Variables|Default|Setvehical_index (Math|Random|RandomIntegerinRange 0 (Utilities|Array|Length (Variables|Default|GetLogs)))))
  (Components|StaticMesh|SetStaticMesh (Variables|Default|GetLog) (Utilities|Array|Get(acopy) (Variables|Default|GetLogs) _output_get))
  (CallFunction|MoveObject))

(event Collision|EventActorBeginOverlap
  (params (OtherActor :type Actor%20Object%20Reference)))

(event EventTick
  (params (DeltaSeconds :type Float%20%28single-precision%29)))

(fn ConstructionScript)
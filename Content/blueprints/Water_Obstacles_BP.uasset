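; Lily pad water obstacle that spins continuously and reacts once when Chicken_Mario_BP overlaps its box.
; The overlap plays a sound, then after a short delay nudges the mesh along local Y and runs the LilyAnimation timeline.
; Timeline updates drift the mesh the opposite way, with a delayed large jump back along Y.
; BeginPlay picks a random mesh branch, but all use Lilpad, which Tick also reapplies every frame.
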(event OnComponentBeginOverlap(Box)
  (params (OverlappedComponent :type Primitive%20Component%20Object%20Reference) (OtherActor :type Actor%20Object%20Reference) (OtherComp :type Primitive%20Component%20Object%20Reference) (OtherBodyIndex :type Integer) (bFromSweep :type Boolean) (SweepResult :type Hit%20Result%20Structure%20%28by%20ref%29))
  (Utilities|Casting|CastToChicken_Mario_BP OtherActor)
  (Utilities|FlowControl|DoOnce false
    (:Completed
      (AddComponent|AddAudioComponent false)
      (Utilities|FlowControl|Delay 0.2)
      (Transformation|AddLocalOffset (Variables|Default|GetWater_Obstacles) (Math|Vector|MakeVector 0.0 (+ 8.0 0.0) 0.0) false false)
      (Timeline|LilyAnimation Play
        (:Update
          (Transformation|AddLocalOffset (Variables|Default|GetWater_Obstacles) (Math|Vector|MakeVector 0.0 (+ -0.1 0.0) 0.0) false false)
          (Utilities|FlowControl|Delay 5.0)
          (Transformation|AddLocalOffset (Variables|Default|GetWater_Obstacles) (Math|Vector|MakeVector 0.0 (+ 1e+02 1e+02) 0.0) false false))))))

(event EventBeginPlay
  (switch int (Math|Random|RandomIntegerinRange 0 2)
    (:0
      (Components|StaticMesh|SetStaticMesh (Variables|Default|GetWater_Obstacles) "/Game/river/lilpad/lilpad.lilpad"))
    (:1
      (Components|StaticMesh|SetStaticMesh (Variables|Default|GetWater_Obstacles) "/Game/river/lilpad/lilpad.lilpad"))
    (:2
      (Components|StaticMesh|SetStaticMesh (Variables|Default|GetWater_Obstacles) "/Game/river/lilpad/lilpad.lilpad"))))

(event Collision|EventActorBeginOverlap
  (params (OtherActor :type Actor%20Object%20Reference)))

(event EventTick
  (params (DeltaSeconds :type Float%20%28single-precision%29))
  (Transformation|AddActorLocalRotation (Components|GetOwner (Variables|Default|GetWater_Obstacles)) (* "0,5.000000, 0" (Variables|Default|GetRotation_Speed)) false false)
  (Components|StaticMesh|SetStaticMesh (Variables|Default|GetWater_Obstacles) "/Game/river/lilpad/lilpad.lilpad"))

(fn ConstructionScript)
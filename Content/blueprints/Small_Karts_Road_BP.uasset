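; Road Blueprint that randomly spawns Small_kart_BP actors once at BeginPlay.
; It loops about once per 900 units between the GrassStart and GrassEnd components, giving each step roughly a 20% spawn chance.
; Every spawn uses the same point, mixing start X and Z with end Y, which is also printed as debug text.
; The out-of-bounds overlap event and construction script are empty.
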(event OnComponentBeginOverlap(PlayerOutOfBounds_Start)
  (params (OverlappedComponent :type Primitive%20Component%20Object%20Reference) (OtherActor :type Actor%20Object%20Reference) (OtherComp :type Primitive%20Component%20Object%20Reference) (OtherBodyIndex :type Integer) (bFromSweep :type Boolean) (SweepResult :type Hit%20Result%20Structure%20%28by%20ref%29)))

(event EventBeginPlay
  (Variables|Default|SetGrassStart (Transformation|GetWorldLocation (Variables|Default|GetGrass_Start)))
  (Variables|Default|SetGrassEnd (Transformation|GetWorldLocation (Variables|Default|GetGrass_End)))
  (for _index (range 0 (Math|Float|Truncate (/ (Math|Vector|Distance(Vector) (Variables|Default|GetGrassStart) (Variables|Default|GetGrassEnd)) 9e+02)))
    (if (> (Math|Random|RandomFloat) 0.8)
      (Game|SpawnActorfromClass "/Game/blueprints/Small_kart_BP.Small_kart_BP_C" (Math|Transform|MakeTransform (Math|Vector|MakeVector (.x (Variables|Default|GetGrassStart)) (.Y (Math|Vector|BreakVector (Variables|Default|GetGrassEnd))) (.z (Variables|Default|GetGrassStart))) "0, 0, 0" "1,1,1") "Undefined" 0 0)))
  (Development|PrintText (Utilities|Text|FormatText (Utilities|Text|ToText(String) (Math|Vector|MakeVector (.x (Variables|Default|GetGrassStart)) (.Y (Math|Vector|BreakVector (Variables|Default|GetGrassEnd))) (.z (Variables|Default|GetGrassStart)))))))

(event Collision|EventActorBeginOverlap
  (params (OtherActor :type Actor%20Object%20Reference)))

(event EventTick
  (params (DeltaSeconds :type Float%20%28single-precision%29)))

(fn ConstructionScript)
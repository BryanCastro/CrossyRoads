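; Goomba is an actor that shows a random vehicle mesh and drives it repeatedly along a spline.
; BeginPlay picks the mesh from the Vehicals array, using an inclusive random range that can overshoot the last index.
; A timeline, rate-scaled by TimeToCompleteS, maps its track to spline distance to set world location and local-space rotation.
; On finish, it snaps the root back to the start and replays.
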(event Custom|MoveObject
  (bind _spline (Variables|Default|Getspline))
  (Components|Timeline|SetPlayRate (Variables|Default|GetMove%20Object%20T) (/ 1.0 (Variables|Default|GetTime%20To%20Complete%28s%29)))
  (bind _move_track (Timeline|Move%20Object%20T Play)
    (:Update
      (Transformation|SetActorTransform (Math|Transform|MakeTransform (Spline|GetLocationatDistanceAlongSpline _spline (Math|Float|Lerp 0.0 (Spline|GetSplineLength _spline) _move_track) "World") (Spline|GetRotationatDistanceAlongSpline _spline (Math|Float|Lerp 0.0 (Spline|GetSplineLength _spline) _move_track) "Local") "1,1,1")))
    (:Finished
      (Transformation|SetWorldLocation (Variables|Default|GetDefaultSceneRoot) (Variables|Default|GetStart_position) false false)
      (Timeline|Move%20Object%20T PlayFromStart))))

(event EventBeginPlay
  (bind _returnvalue (Actor|GetActorOfClass "/Game/blueprints/Vehicle_BP.Vehicle_BP_C"))
  (Variables|Default|SetNewVar_0 _returnvalue)
  (Variables|Default|SetStart_position (Transformation|GetWorldLocation (Variables|Default|GetDefaultSceneRoot)))
  (bind _output_get (Variables|Default|Setvehical_index (Math|Random|RandomIntegerinRange 0 (Utilities|Array|Length (Variables|Default|GetVehicals)))))
  (Components|StaticMesh|SetStaticMesh (Variables|Default|GetCar) (Utilities|Array|Get(acopy) (Variables|Default|GetVehicals) _output_get))
  (CallFunction|MoveObject))

(event Collision|EventActorBeginOverlap
  (params (OtherActor :type Actor%20Object%20Reference)))

(event EventTick
  (params (DeltaSeconds :type Float%20%28single-precision%29)))

(fn ConstructionScript)
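; Grass obstacle actor that appears as a random small tree, rock, tree or coin and acts as a pickup for the chicken player.
; BeginPlay picks the static mesh at random and applies a scale delta for the coin.
; Box overlap with Chicken_Mario_BP, regardless of the chosen mesh, destroys the actor, adds to the player's points and coin score, then adds an audio component.
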(event OnComponentBeginOverlap(box)
  (params (OverlappedComponent :type Primitive%20Component%20Object%20Reference) (OtherActor :type Actor%20Object%20Reference) (OtherComp :type Primitive%20Component%20Object%20Reference) (OtherBodyIndex :type Integer) (bFromSweep :type Boolean) (SweepResult :type Hit%20Result%20Structure%20%28by%20ref%29))
  (bind _aschicken_mario_bp (Utilities|Casting|CastToChicken_Mario_BP OtherActor))
  (Actor|DestroyActor)
  (Default|AddPoints _aschicken_mario_bp 1)
  (Default|AddCoinScore _aschicken_mario_bp 1)
  (AddComponent|AddAudioComponent false))

(event EventBeginPlay
  (bind _grass_obstacles (Variables|Default|GetGrass_Obstacles))
  (switch int (Math|Random|RandomIntegerinRange 0 3)
    (:0
      (Components|StaticMesh|SetStaticMesh (Variables|Default|GetGrass_Obstacles) "/Game/Tree_v2/tree_small_v2.tree_small_v2"))
    (:1
      (Components|StaticMesh|SetStaticMesh (Variables|Default|GetGrass_Obstacles) "/Game/landscape/rock.rock"))
    (:2
      (Components|StaticMesh|SetStaticMesh (Variables|Default|GetGrass_Obstacles) "/Game/Tree_v2/tree_v2.tree_v2"))
    (:3
      (Components|StaticMesh|SetStaticMesh _grass_obstacles "/Game/coin/coin.coin")
      (Class|SceneComponent|AddLocalTransform _grass_obstacles (Math|Transform|MakeTransform "0, 0, 0" "0, 0, 0" "50.000000,50.000000,50.000000") false false))))

(event Collision|EventActorBeginOverlap
  (params (OtherActor :type Actor%20Object%20Reference)))

(event EventTick
  (params (DeltaSeconds :type Float%20%28single-precision%29)))

(fn ConstructionScript)
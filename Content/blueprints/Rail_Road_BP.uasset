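; Rail road lane actor that spawns a train and lights up three coin blocks in response to overlaps.
; On BeginPlay it caches both grass end locations and spawns Train_BP at the start's X and Z with the end's Y.
; Each coin block has paired out-of-bounds volumes: entering one applies the lit material, leaving the other restores the unlit one.
; An unfinished random loop along the track length is left disconnected.
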(event OnComponentBeginOverlap(PlayerOutOfBounds_End_mid)
  (params (OverlappedComponent :type Primitive%20Component%20Object%20Reference) (OtherActor :type Actor%20Object%20Reference) (OtherComp :type Primitive%20Component%20Object%20Reference) (OtherBodyIndex :type Integer) (bFromSweep :type Boolean) (SweepResult :type Hit%20Result%20Structure%20%28by%20ref%29)))

(event OnComponentEndOverlap(PlayerOutOfBounds_End_start)
  (params (OverlappedComponent :type Primitive%20Component%20Object%20Reference) (OtherActor :type Actor%20Object%20Reference) (OtherComp :type Primitive%20Component%20Object%20Reference) (OtherBodyIndex :type Integer))
  (Rendering|Material|CreateDynamicMaterialInstance (Variables|Default|Getcoinblock_Start) 0 "/Game/coinblock/coinblock_unlit_mat_Inst.coinblock_unlit_mat_Inst" "None" :!class /Script/Engine.PrimitiveComponent))

(event OnComponentEndOverlap(PlayerOutOfBounds_End)
  (params (OverlappedComponent :type Primitive%20Component%20Object%20Reference) (OtherActor :type Actor%20Object%20Reference) (OtherComp :type Primitive%20Component%20Object%20Reference) (OtherBodyIndex :type Integer))
  (Rendering|Material|CreateDynamicMaterialInstance (Variables|Default|Getcoinblock_End) 0 "/Game/coinblock/coinblock_unlit_mat_Inst.coinblock_unlit_mat_Inst" "None" :!class /Script/Engine.PrimitiveComponent))

(event OnComponentBeginOverlap(PlayerOutOfBounds_Start)
  (params (OverlappedComponent :type Primitive%20Component%20Object%20Reference) (OtherActor :type Actor%20Object%20Reference) (OtherComp :type Primitive%20Component%20Object%20Reference) (OtherBodyIndex :type Integer) (bFromSweep :type Boolean) (SweepResult :type Hit%20Result%20Structure%20%28by%20ref%29))
  (Rendering|Material|CreateDynamicMaterialInstance (Variables|Default|Getcoinblock_End) 0 "/Game/coinblock/coinblock_lit_mat_Inst.coinblock_lit_mat_Inst" "None" :!class /Script/Engine.PrimitiveComponent))

(event OnComponentBeginOverlap(PlayerOutOfBounds_Start_mid)
  (params (OverlappedComponent :type Primitive%20Component%20Object%20Reference) (OtherActor :type Actor%20Object%20Reference) (OtherComp :type Primitive%20Component%20Object%20Reference) (OtherBodyIndex :type Integer) (bFromSweep :type Boolean) (SweepResult :type Hit%20Result%20Structure%20%28by%20ref%29))
  (Rendering|Material|CreateDynamicMaterialInstance (Variables|Default|Getcoinblock) 0 "/Game/coinblock/coinblock_lit_mat_Inst.coinblock_lit_mat_Inst" "None" :!class /Script/Engine.PrimitiveComponent))

(event OnComponentBeginOverlap(PlayerOutOfBounds_Start_start)
  (params (OverlappedComponent :type Primitive%20Component%20Object%20Reference) (OtherActor :type Actor%20Object%20Reference) (OtherComp :type Primitive%20Component%20Object%20Reference) (OtherBodyIndex :type Integer) (bFromSweep :type Boolean) (SweepResult :type Hit%20Result%20Structure%20%28by%20ref%29))
  (Rendering|Material|CreateDynamicMaterialInstance (Variables|Default|Getcoinblock_Start) 0 "/Game/coinblock/coinblock_lit_mat_Inst.coinblock_lit_mat_Inst" "None" :!class /Script/Engine.PrimitiveComponent))

(event OnComponentBeginOverlap(PlayerOutOfBounds_End_start)
  (params (OverlappedComponent :type Primitive%20Component%20Object%20Reference) (OtherActor :type Actor%20Object%20Reference) (OtherComp :type Primitive%20Component%20Object%20Reference) (OtherBodyIndex :type Integer) (bFromSweep :type Boolean) (SweepResult :type Hit%20Result%20Structure%20%28by%20ref%29)))

(event OnComponentEndOverlap(PlayerOutOfBounds_End_mid)
  (params (OverlappedComponent :type Primitive%20Component%20Object%20Reference) (OtherActor :type Actor%20Object%20Reference) (OtherComp :type Primitive%20Component%20Object%20Reference) (OtherBodyIndex :type Integer))
  (Rendering|Material|CreateDynamicMaterialInstance (Variables|Default|Getcoinblock) 0 "/Game/coinblock/coinblock_unlit_mat_Inst.coinblock_unlit_mat_Inst" "None" :!class /Script/Engine.PrimitiveComponent))

(event EventBeginPlay
  (Variables|Default|SetRailRoadStart (Transformation|GetWorldLocation (Variables|Default|GetGrass_Start)))
  (Variables|Default|SetRailRoadEnd (Transformation|GetWorldLocation (Variables|Default|GetGrass_End)))
  (Game|SpawnActorfromClass "/Game/blueprints/Train_BP.Train_BP_C" (Math|Transform|MakeTransform (Math|Vector|MakeVector (.x (Variables|Default|GetRailRoadStart)) (.Y (Math|Vector|BreakVector (Variables|Default|GetRailRoadEnd))) (.z (Variables|Default|GetRailRoadStart))) "0, 0, 0" "1,1,1") "Undefined" 0 0))

(event Collision|EventActorBeginOverlap
  (params (OtherActor :type Actor%20Object%20Reference)))

(event EventTick
  (params (DeltaSeconds :type Float%20%28single-precision%29)))

(fn ConstructionScript)
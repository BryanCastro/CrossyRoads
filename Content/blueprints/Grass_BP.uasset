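; Grass strip actor that randomly scatters Grass_Obstacles_BP actors along its length when play begins.
; BeginPlay reads the GrassStart and GrassEnd world locations and divides their distance into 100-unit slots.
; Each slot has about a 20% chance to spawn an obstacle, stepping along positive world Y from one slot behind GrassStart.
; A debug print shows the last computed position after the loop.
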(event EventBeginPlay
  (Variables|Default|SetGrassStart (Transformation|GetWorldLocation (Variables|Default|GetGrass_Start)))
  (Variables|Default|SetGrassEnd (Transformation|GetWorldLocation (Variables|Default|GetGrass_End)))
  (for _index (range 0 (Math|Float|Truncate (/ (Math|Vector|Distance(Vector) (Variables|Default|GetGrassStart) (Variables|Default|GetGrassEnd)) 1e+02)))
    (if (> (Math|Random|RandomFloat) 0.8)
      (Game|SpawnActorfromClass "/Game/blueprints/Grass_Obstacles_BP.Grass_Obstacles_BP_C" (Math|Transform|MakeTransform (Math|Vector|MakeVector (.x (Variables|Default|GetGrassStart)) (- (+ (* _index 1e+02) (.Y (Math|Vector|BreakVector (Variables|Default|GetGrassStart)))) 1e+02) (.z (Variables|Default|GetGrassStart))) "0, 0, 0" "1,1,1") "Undefined" 0 0)))
  (Development|PrintText (Utilities|Text|FormatText (Utilities|Text|ToText(String) (Math|Vector|MakeVector (.x (Variables|Default|GetGrassStart)) (- (+ (* _index 1e+02) (.Y (Math|Vector|BreakVector (Variables|Default|GetGrassStart)))) 1e+02) (.z (Variables|Default|GetGrassStart)))))))

(event Collision|EventActorBeginOverlap
  (params (OtherActor :type Actor%20Object%20Reference)))

(event EventTick
  (params (DeltaSeconds :type Float%20%28single-precision%29)))

(fn ConstructionScript)
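; Kart obstacle actor that spawns with a random mesh and squashes the Chicken_Mario_BP player when it enters the kill zone.
; A timeline repeatedly moves it along a spline, randomly choosing a flipped, offset start or the default one for each run.
; KillZone snaps the chicken to the kart and flattens its scale, while other triggers disable kart collision or add one-shot audio, picked by fresh random rolls rather than the displayed mesh.
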(event OnComponentBeginOverlap(killZone)
  (params (OverlappedComponent :type Primitive%20Component%20Object%20Reference) (OtherActor :type Actor%20Object%20Reference) (OtherComp :type Primitive%20Component%20Object%20Reference) (OtherBodyIndex :type Integer) (bFromSweep :type Boolean) (SweepResult :type Hit%20Result%20Structure%20%28by%20ref%29))
  (bind _defaultsceneroot (Variables|Default|GetDefaultSceneRoot))
  (bind _returnvalue (Transformation|GetWorldLocation _defaultsceneroot))
  (bind _aschicken_mario_bp (Utilities|Casting|CastToChicken_Mario_BP OtherActor))
  (Variables|Default|SetChicken 0)
  (Transformation|SetActorTransform _aschicken_mario_bp (Math|Transform|MakeTransform (Math|Vector|MakeVector (.x _returnvalue) (.y _returnvalue) 1258.0) "0, 0, 0" "1,0.200000,1.000000")))

(event OnComponentBeginOverlap(DisableCollision)
  (params (OverlappedComponent :type Primitive%20Component%20Object%20Reference) (OtherActor :type Actor%20Object%20Reference) (OtherComp :type Primitive%20Component%20Object%20Reference) (OtherBodyIndex :type Integer) (bFromSweep :type Boolean) (SweepResult :type Hit%20Result%20Structure%20%28by%20ref%29))
  (Collision|SetCollisionEnabled (Variables|Default|GetCar) "NoCollision")
  (Variables|Default|SetDisableCollision 0))

(event OnComponentBeginOverlap(Yoshi)
  (params (OverlappedComponent :type Primitive%20Component%20Object%20Reference) (OtherActor :type Actor%20Object%20Reference) (OtherComp :type Primitive%20Component%20Object%20Reference) (OtherBodyIndex :type Integer) (bFromSweep :type Boolean) (SweepResult :type Hit%20Result%20Structure%20%28by%20ref%29))
  (Utilities|Casting|CastToChicken_Mario_BP OtherActor)
  (Utilities|FlowControl|DoOnce false
    (:Completed
      (if (== (Utilities|Array|Get(acopy) (Variables|Default|GetVehicals) (Math|Random|RandomIntegerinRange 0 1)) "/Game/characters/character_karts/yoshikart.yoshikart")
        (AddComponent|AddAudioComponent false)
        (elif (== (Utilities|Array|Get(acopy) (Variables|Default|GetVehicals) (Math|Random|RandomIntegerinRange 1 2)) "/Game/characters/character_karts/luigikart.luigikart")
          (AddComponent|AddAudioComponent false)
          (else
            (AddComponent|AddAudioComponent false)))))))

(event Custom|MoveObject
  (bind _spline (Variables|Default|Getspline))
  (bind _start_position (Variables|Default|GetStart_position))
  (Components|Timeline|SetPlayRate (Variables|Default|GetMove%20Object%20T) (/ 1.0 (Variables|Default|GetTime%20To%20Complete%28s%29)))
  (if (> (Math|Random|RandomInteger 3) 0) :!label _label
    (Variables|Default|SetRotation "0,180.000000, 0")
    (Transformation|SetActorTransform (Math|Transform|MakeTransform (+ _start_position "0,-2000.000000, 0") "0,180.000000, 0" "1,1,1"))
    (bind _move_track (Timeline|Move%20Object%20T PlayFromStart)
      (:Update
        (Transformation|SetActorLocation (Spline|GetLocationatDistanceAlongSpline _spline (Math|Float|Lerp 0.0 (Spline|GetSplineLength _spline) _move_track) "World") false false))
      (:Finished
        (Transformation|SetWorldLocation (Variables|Default|GetDefaultSceneRoot) _start_position false false)
        (Utilities|FlowControl|Delay 0.2)
        (goto _label)))
    (else
      (Variables|Default|SetRotation "0, 0, 0")
      (Transformation|SetActorTransform (Math|Transform|MakeTransform _start_position "0, 0, 0" "1,1,1"))
      (Timeline|Move%20Object%20T PlayFromStart))))

(event EventBeginPlay
  (bind _returnvalue (Actor|GetActorOfClass "/Game/blueprints/Vehicle_BP.Vehicle_BP_C"))
  (Variables|Default|SetNewVar_0 _returnvalue)
  (Variables|Default|SetStart_position (Transformation|GetWorldLocation (Variables|Default|GetDefaultSceneRoot)))
  (bind _output_get (Variables|Default|Setvehical_index (Math|Random|RandomIntegerinRange 0 (Utilities|Array|Length (Variables|Default|GetVehicals)))))
  (Components|StaticMesh|SetStaticMesh (Variables|Default|GetCar) (Utilities|Array|Get(acopy) (Variables|Default|GetVehicals) _output_get))
  (CallFunction|MoveObject))

(event Collision|EventActorBeginOverlap
  (params (OtherActor :type Actor%20Object%20Reference)))

(event EventTick
  (params (DeltaSeconds :type Float%20%28single-precision%29)))

(fn ConstructionScript)
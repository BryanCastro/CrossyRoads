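; Lane generator that builds an endless Crossy Road-style track ahead of the chicken player in 16-lane chunks.
; On BeginPlay it spawns evenly spaced lanes along X from Ground: a grass block, a water block, then randomly chosen kart or rail roads.
; Each random road also gets a detection actor bound to an overlap event.
; The first Chicken_Mario_BP overlap passes a DoOnce and spawns another generator one chunk ahead, chaining the track.
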(event Custom|OnActorBeginOverlap_Event_0
  (params (OverlappedActor :type Actor%20Object%20Reference) (OtherActor :type Actor%20Object%20Reference))
  (bind _ground (Variables|Default|GetGround))
  (bind _returnvalue (Transformation|GetWorldLocation _ground))
  (Utilities|Casting|CastToChicken_Mario_BP OtherActor)
  (Utilities|FlowControl|DoOnce false
    (:Completed
      (bind _output_get (Variables|Default|SetSpawnLaneLocation (Math|Vector|MakeVector (+ 1.6e+03 (.x _returnvalue)) (.y _returnvalue) (.z _returnvalue))))
      (Game|SpawnActorfromClass "Lane_Generator_BP_C" (Math|Transform|MakeTransform _output_get "0, 0, 0" "1,1,1") "Undefined" 0 0))))

(event EventBeginPlay
  (bind _ground (Variables|Default|GetGround))
  (bind _returnvalue (Transformation|GetWorldLocation _ground))
  (for _index (range 0 15)
    (Variables|Default|SetSpawnLaneLocation (Math|Vector|MakeVector (+ (* _index 1e+02) (.x _returnvalue)) (.y _returnvalue) (.z _returnvalue)))
    (if (Math|Integer|InRange(Integer) _index 0 6)
      (Game|SpawnActorfromClass "/Game/blueprints/Grass_BP.Grass_BP_C" (Math|Transform|MakeTransform (Variables|Default|GetSpawnLaneLocation) "0, 0, 0" "1,1,1") "Undefined" 0 0)
      (elif (Math|Integer|InRange(Integer) _index 7 9)
        (Game|SpawnActorfromClass "/Game/blueprints/Water_BP.Water_BP_C" (Math|Transform|MakeTransform (Variables|Default|GetSpawnLaneLocation) "0, 0, 0" "1,1,1") "Undefined" 0 0)
        (else
          (if (Math|Integer|InRange(Integer) _index 10 15)
            (switch int (Math|Random|RandomIntegerinRange 0 3)
              (:0
                (Game|SpawnActorfromClass "/Game/blueprints/Mid_Kart_Road_BP.Mid_Kart_Road_BP_C" (Math|Transform|MakeTransform (Variables|Default|GetSpawnLaneLocation) "0, 0, 0" "1,1,1") "Undefined" 0 0))
              (:1
                (Game|SpawnActorfromClass "/Game/blueprints/Small_Karts_Road_BP.Small_Karts_Road_BP_C" (Math|Transform|MakeTransform (Variables|Default|GetSpawnLaneLocation) "0, 0, 0" "1,1,1") "Undefined" 0 0))
              (:2
                (Game|SpawnActorfromClass "/Game/blueprints/Big_Karts_Road_BP.Big_Karts_Road_BP_C" (Math|Transform|MakeTransform (Variables|Default|GetSpawnLaneLocation) "0, 0, 0" "1,1,1") "Undefined" 0 0))
              (:3
                (Game|SpawnActorfromClass "/Game/blueprints/Rail_Road_BP.Rail_Road_BP_C" (Math|Transform|MakeTransform (Variables|Default|GetSpawnLaneLocation) "0, 0, 0" "1,1,1") "Undefined" 0 0))))
          (bind _returnvalue_2 (Game|SpawnActorfromClass "/Game/blueprints/Detection_To_Respawn_Lanes_BP.Detection_To_Respawn_Lanes_BP_C" (Math|Transform|MakeTransform (Variables|Default|GetSpawnLaneLocation) "0, 0, 0" "1,1,1") "Undefined" 0 0))
          (Collision|BindEventtoOnActorBeginOverlap _returnvalue_2 (delegate Custom|OnActorBeginOverlap_Event_0)))))))

(event Collision|EventActorBeginOverlap
  (params (OtherActor :type Actor%20Object%20Reference)))

(event EventTick
  (params (DeltaSeconds :type Float%20%28single-precision%29)))

(fn ConstructionScript)
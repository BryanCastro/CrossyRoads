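; Player character for a hop-based game, moving a Mario model in short launched jumps along forward and right axes.
; Input past a deadzone launches the character, adds an audio component, awards a point and plays a timeline turning the model toward travel.
; A DoOnce-gated half-second cooldown blocks repeated hops.
; A HUB widget created on BeginPlay displays the score and coin count updated through AddPoints and AddCoinScore.
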(event Custom|AddPoints
  (params (Point%20Value :type Integer))
  (Variables|Default|SetPoints (+ Point%20Value (Variables|Default|GetPoints)))
  (Default|UpdateScore (Variables|Default|GetUI) (Variables|Default|GetPoints)))

(event Custom|MovementCooldown
  (Utilities|FlowControl|DoOnce false :!label _label
    (:Completed
      (Variables|Default|SetCanmove false)
      (Utilities|FlowControl|Delay 0.5)
      (Variables|Default|SetCanmove true)
      (goto _label Reset))))

(event Custom|AddCoinScore
  (params (CoinPoints :type Integer))
  (Variables|Default|SetCoinPoints (+ CoinPoints (Variables|Default|GetCoinPoints)))
  (Default|UpdateCoinScore (Variables|Default|GetUI) (Variables|Default|GetCoinPoints)))

(event Collision|EventActorBeginOverlap
  (params (OtherActor :type Actor%20Object%20Reference)))

(event EventTick
  (params (DeltaSeconds :type Float%20%28single-precision%29)))

(event EventBeginPlay
  (bind _returnvalue (UserInterface|CreateWidget "/Game/UI/HUB.HUB_C"))
  (bind _output_get (Variables|Default|SetUI _returnvalue))
  (UserInterface|Viewport|AddtoViewport _output_get 0))

(event Input|AxisEvents|InputAxisMoveForward
  (params (AxisValue :type Float%20%28single-precision%29))
  (bind _mario (Variables|Default|GetMario))
  (bind _mario_2 (Variables|Default|GetMario))
  (if (and (> (Math|Float|Absolute(Float) AxisValue) 0.3) (Variables|Default|GetCanmove))
    (CallFunction|MovementCooldown)
    (Character|LaunchCharacter (Math|Vector|MakeVector (* AxisValue 225.0) 0.0 1.9e+02) false false)
    (CallFunction|AddPoints 1)
    (AddComponent|AddAudioComponent false)
    (if (> AxisValue 0.3)
      (bind _newtrack_0 (Timeline|Timeline_0 PlayFromStart)
        (:Update
          (Transformation|SetWorldRotation _mario (Math|Rotator|Lerp(Rotator) (Transformation|GetWorldRotation _mario) "0.000000,90.000000,90.000000" _newtrack_0 true) false false)))
      (else
        (bind _newtrack_0_2 (Timeline|Timeline_1 PlayFromStart)
          (:Update
            (Transformation|SetWorldRotation _mario_2 (Math|Rotator|Lerp(Rotator) (Transformation|GetWorldRotation _mario_2) "0.000000,270.000000,90.000000" _newtrack_0_2 true) false false)))))))

(event Input|AxisEvents|InputAxisMoveRight
  (params (AxisValue :type Float%20%28single-precision%29))
  (bind _mario (Variables|Default|GetMario))
  (bind _mario_2 (Variables|Default|GetMario))
  (if (and (> (Math|Float|Absolute(Float) AxisValue) 0.3) (Variables|Default|GetCanmove))
    (CallFunction|MovementCooldown)
    (Character|LaunchCharacter (Math|Vector|MakeVector 0.0 (* AxisValue 225.0) 1.9e+02) false false)
    (CallFunction|AddPoints 1)
    (AddComponent|AddAudioComponent false)
    (if (> AxisValue 0.3)
      (bind _newtrack_0 (Timeline|Timeline_2 PlayFromStart)
        (:Update
          (Transformation|SetWorldRotation _mario_2 (Math|Rotator|Lerp(Rotator) (Transformation|GetWorldRotation _mario_2) "0.000000,180.000000,90.000000" _newtrack_0 true) false false)))
      (else
        (bind _newtrack_0_2 (Timeline|Timeline_3 PlayFromStart)
          (:Update
            (Transformation|SetWorldRotation _mario (Math|Rotator|Lerp(Rotator) (Transformation|GetWorldRotation _mario) "0.000000,360.000000,90.000000" _newtrack_0_2 true) false false)))))))

(fn ConstructionScript)
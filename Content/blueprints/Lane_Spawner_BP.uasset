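; Spawner actor that builds a chained track of Lane_BP lanes, starting with a small initial set on BeginPlay.
; The first lane spawns at the player controller's location, and each following one at the newest lane's LaneSpawnPoint.
; Each lane receives a reference back to the spawner, which tracks the newest lane.
; RandomizeLanes sets a random mesh on the Lane component but is not called here.
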(event EventBeginPlay
  (CallFunction|SpawnInitialLanes))

(event Collision|EventActorBeginOverlap
  (params (OtherActor :type Actor%20Object%20Reference)))

(event EventTick
  (params (DeltaSeconds :type Float%20%28single-precision%29)))

(fn ConstructionScript)

(fn SpawnLane
  (params (SpawnLocation :type Vector))
  (bind _returnvalue (Game|SpawnActorfromClass "/Game/blueprints/Lane_BP.Lane_BP_C" (Math|Transform|MakeTransform SpawnLocation "0, 0, 0" "1,1,1") "Undefined" 0 0))
  (bind _output_get (Variables|Default|SetNewestLane _returnvalue))
  (Variables|/Game/blueprints/Lane_BP.Lane_BP_C|SetLaneSpawner _output_get self))

(fn SpawnLaneatSpawnPoint
  (CallFunction|SpawnLane (Transformation|GetWorldLocation (Variables|/Game/blueprints/Lane_BP.Lane_BP_C|GetLaneSpawnPoint (Variables|Default|GetNewestLane)))))

(fn SpawnInitialLanes
  (for _index (range 0 2)
    (Utilities|IsValid (Variables|Default|GetNewestLane)
      (:Is%20Valid
        (CallFunction|SpawnLaneatSpawnPoint))
      (:Is%20Not%20Valid
        (CallFunction|SpawnLane (Transformation|GetActorLocation (Game|GetPlayerController 0)))))))

(fn RandomizeLanes
  (bind _returnvalue (Actor|GetActorOfClass "/Game/blueprints/Lane_BP.Lane_BP_C"))
  (Variables|Default|SetNewVar_1 _returnvalue)
  (bind _output_get (Variables|Default|Setlane_Index (Math|Random|RandomIntegerinRange 0 (Utilities|Array|Length (Variables|Default|GetLanes)))))
  (Components|StaticMesh|SetStaticMesh (Variables|Default|Getlane) (Utilities|Array|Get(acopy) (Variables|Default|GetLanes) _output_get)))